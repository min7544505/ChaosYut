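; BP_RoadBase is a clickable board space that pieces move to, apparently for a Yut game.
; Clicking its mesh tells PC_Yut to move the selected piece to this road.
; Its ReachableSign starts hidden and toggles through SetReachableSignVisibility; its Tick yaw rotation is multiplied by zero, so it does not spin.
; The construction script sets PieceLocation's height to the top of the mesh's local bounds.
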(event `self.ReceiveBeginPlay`
  (`self.SetReachableSignVisibility` false))

(event `self.ReceiveTick`
  (params (DeltaSeconds :type "Float (single-precision)"))
  (`SceneComponent.K2_AddWorldRotation` (`self.ReachableSign`) (`KismetMathLibrary.MakeRotator` 0.0 0.0 (* DeltaSeconds 0.0)) false false))

(event `self.StaticMesh.OnClicked`
  (params (TouchedComponent :type "PrimitiveComponent Object Reference") (ButtonPressed :type "Key Structure"))
  (bind _aspc_yut (cast `/Game/UI/PC_Yut` (`GameplayStatics.GetPlayerController` 0)))
  (`/Game/UI/PC_Yut.MoveSelectedPieceToRoad` _aspc_yut self))

(fn `SetReachableSignVisibility`
  (params (bNewVisibility :type Boolean))
  (`SceneComponent.SetVisibility` (`self.ReachableSign`) bNewVisibility false))

(fn `UserConstructionScript`
  (`SceneComponent.K2_SetRelativeLocation` (`self.PieceLocation`) (`KismetMathLibrary.MakeVector` 0.0 0.0 (.z (`.Max` (`StaticMeshComponent.GetLocalBounds` (`self.StaticMesh`))))) false false))