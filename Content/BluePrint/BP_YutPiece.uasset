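; BP_YutPiece is a clickable game piece for a Yut board game that moves between road spaces on the board.
; On BeginPlay it hides its selection cone and takes the board's Road00M child actor as its current road.
; Clicking the mesh passes the piece to PC_Yut for selection, while MoveToRoad snaps it to a road's PieceLocation.
; The selection cone spins continuously on Tick and is shown or hidden through SetSelectedMarkVisibility.
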(event `self.ReceiveBeginPlay`
  (`self.SetSelectedMarkVisibility` false)
  (bind _outactors (`GameplayStatics.GetAllActorsOfClass` "/Game/Blueprint/BP_YutBoard.BP_YutBoard_C"))
  (if (>= (`KismetArrayLibrary.Array_Length` _outactors) 1)
    (bind _asbp_road_base (cast `/Game/Blueprint/BP_RoadBase` (`ChildActorComponent.ChildActor` (`/Game/Blueprint/BP_YutBoard.Road00_M` (`|GetArrayItem` _outactors)))))
    (set `self.CurRoad` _asbp_road_base)))

(event `self.ReceiveTick`
  (params (DeltaSeconds :type "Float (single-precision)"))
  (`SceneComponent.K2_AddWorldRotation` (`self.Shape_Cone`) (`KismetMathLibrary.MakeRotator` 0.0 0.0 (* DeltaSeconds 180.0)) false false))

(event `self.StaticMesh.OnClicked`
  (params (TouchedComponent :type "PrimitiveComponent Object Reference") (ButtonPressed :type "Key Structure"))
  (bind _aspc_yut (cast `/Game/UI/PC_Yut` (`GameplayStatics.GetPlayerController` 0)))
  (`/Game/UI/PC_Yut.SelectYutPiece` _aspc_yut self))

(fn `MoveToRoad`
  (params (DestRoad :type "/Game/Blueprint/BP_RoadBase Object Reference"))
  (`/Engine/EditorBlueprintResources/StandardMacros.IsValid` DestRoad
    (:`Is Valid`
      (bind _output_get (set `self.CurRoad` DestRoad))
      (`self.K2_SetActorLocation` (`SceneComponent.K2_GetComponentLocation` (`/Game/Blueprint/BP_RoadBase.PieceLocation` _output_get))))))

(fn `SetSelectedMarkVisibility`
  (params (bNewVisibility :type Boolean))
  (`SceneComponent.SetVisibility` (`self.Shape_Cone`) bNewVisibility true))

(fn `UserConstructionScript`)