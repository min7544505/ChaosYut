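; Board actor for a Yut game that wires its child-actor road spaces into a linked path graph.
; On BeginPlay it collects them as BP_RoadBase into Roads and links each Prev/Next by array index.
; It then hand-patches out-of-order links, assigns shortcuts on branch roads, and runs a pass meant to give merge roads a second previous road.
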(event `self.ReceiveBeginPlay`
  (`|ExecutionSequence`
    (:`then_0`
      ; Roads에 RoadBase 형태로 담기
      (bind _output_get (set `self.RoadChildActor` (`|MakeArray` (`self.Road00_M`) (`self.Road01`) (`self.Road02`) (`self.Road03`) (`self.Road04`) (`self.Road05_B`) (`self.Road06`) (`self.Road07`) (`self.Road08`) (`self.Road09`) (`self.Road10_B`) (`self.Road11`) (`self.Road12`) (`self.Road13`) (`self.Road14`) (`self.Road15_M`) (`self.Road16`) (`self.Road17`) (`self.Road18`) (`self.Road19`) (`self.Road20`) (`self.Road21`) (`self.Road22_J`) (`self.Road23`) (`self.Road24`) (`self.Road25`) (`self.Road26`) (`self.Road27`) (`self.Road28`))))
      (for _array_element _output_get
        (bind _asbp_road_base (cast `/Game/Blueprint/BP_RoadBase` (`ChildActorComponent.ChildActor` _array_element)))
        (`KismetArrayLibrary.Array_Add` (`self.Roads`) _asbp_road_base)))
    (:`then_1`
      ; 연결된 길 초기화
      ;; 인덱스 순서에 맞게 연결된 길들 초기화
      (for (_array_element_2 _array_index) (`self.Roads`)
        (`self.InitLinkedRoadInOrder` _array_element_2 _array_index))
      ;; 인덱스와 순서가 맞지 않은 길들은 수동으로 초기화
      (`self.SetNextRoad` (`|GetArrayItem` (`self.Roads`) 24) 15)
      (`self.SetNextRoad` (`|GetArrayItem` (`self.Roads`) 28) 0)
      (`self.SetNextRoad` (`|GetArrayItem` (`self.Roads`) 26) 22)
      (`self.SetNextRoad` (`|GetArrayItem` (`self.Roads`) 19) 0))
    (:`then_2`
      ; 갈림길에 필요한 지름길 초기화
      (`self.SetBranchRoadShortCut` (`self.Road20`) (`self.Road05_B`))
      (`self.SetBranchRoadShortCut` (`self.Road25`) (`self.Road10_B`)))
    (:`then_3`
      ; 합류점에 필요한 두 번째 이전길 초기화
      (`self.SetMergeRoadPrev2` (`|GetArrayItem` (`self.Roads`) 15) 24)
      (`self.SetMergeRoadPrev2` (`|GetArrayItem` (`self.Roads`) 28) 24))))

(fn `UserConstructionScript`)